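; Board actor for a board game that builds a tiled grid with a background and two team zones on BeginPlay.
; SetBoardSize sizes a 2D array of tile structs from BoardSize, spawns a scaled BP_Tile per cell and stores its reference, then spawns a centred, bordered background.
; SetTeamAffiliationTiles assigns team 1 (blue) to the first rows and team 2 (red) to the last, if the board has enough rows.
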(event `self.ReceiveBeginPlay`
  (`self.SetBoardSize`)
  (`self.SetTeamAffiliationTiles`))

(fn `SetBoardSize`
  (bind _board2d (`self.Board2D`))
  (bind (_boardsize_x _boardsize_y) (break `/Game/AlgorithmBoardGame/Blueprints/Structs/F_IntVector2D` (`self.BoardSize`)))
  (bind _backgroundborderwidth (`self.BackgroundBorderWidth`))
  (bind _tilesize (`self.TileSize`))
  (bind _tilepadding (`self.TilePadding`))
  (bind (_boardsize_x_2 _boardsize_y_2) (break `/Game/AlgorithmBoardGame/Blueprints/Structs/F_IntVector2D` (`self.BoardSize`)))
  (bind (_x _y) (break `/Game/AlgorithmBoardGame/Blueprints/Structs/F_IntVector2D` (`self.BoardSize`)))
  (bind _returnvalue (/ (`self.TileSize`) 100.0))
  (bind _returnvalue_2 (+ (`self.TileSize`) (`self.TilePadding`)))
  ;[1 1 1] Resizing Board2D
  (`KismetArrayLibrary.Array_Resize` (`self.Board2D`) _y)
  (for (_ _array_index) (`self.Board2D`)
    (`KismetArrayLibrary.Array_Resize` (`.1DBoard_4_A8DABEF5403C21CC9E4A7485542F37BF` (break `/Game/AlgorithmBoardGame/Blueprints/Structs/F_Board1D` (`|GetArrayItem` _board2d _array_index))) _x)
    (bind _1dboard (break `/Game/AlgorithmBoardGame/Blueprints/Structs/F_Board1D` (`|GetArrayItem` _board2d _array_index)))
    ;[0.6875 1 0.7233] Create Tile Objects
    (for (_ _array_index_2) _1dboard
      (bind _returnvalue_3 (`|SpawnActorFromClass` "/Game/AlgorithmBoardGame/Blueprints/BP_Tile.BP_Tile_C" (`KismetMathLibrary.MakeTransform` (`KismetMathLibrary.MakeVector` (* _array_index_2 (+ _tilesize _tilepadding)) (* _array_index (+ _tilesize _tilepadding)) 2.0) (struct) (`KismetMathLibrary.MakeVector` _returnvalue _returnvalue 0.04)) "Undefined" "MultiplyWithRoot" null null))
      (setmembers `/Game/AlgorithmBoardGame/Blueprints/Structs/F_BoardTile` :`StructRef` (`|GetArrayItem` _1dboard _array_index_2) :`TileObject` _returnvalue_3)))
  ;[0.9057 0.7914 1] Create Board Background Object
  (`|SpawnActorFromClass` "/Game/AlgorithmBoardGame/Blueprints/BP_BoardBackground.BP_BoardBackground_C" (`KismetMathLibrary.MakeTransform` (/ (`KismetMathLibrary.MakeVector` (* _returnvalue_2 (- _boardsize_x 1)) (* _returnvalue_2 (- _boardsize_y 1))) (2.0 2.0 1.0)) (struct) (/ (`KismetMathLibrary.MakeVector` (+ (* _returnvalue_2 _boardsize_x_2) _backgroundborderwidth) (+ (* _returnvalue_2 _boardsize_y_2) _backgroundborderwidth) 1.0) (100.0 100.0 1.0))) "Undefined" "MultiplyWithRoot" null null))

(fn `SetTeamAffiliationTiles`
  (bind _teamaffiliationrowcount (`self.TeamAffiliationRowCount`))
  (bind _returnvalue (`KismetArrayLibrary.Array_Length` (`self.Board2D`)))
  ;[1 1 1] Check if Board is large enough to create Team Affiliation Tiles
  (if (<= (* (`self.TeamAffiliationRowCount`) 2) _returnvalue)
    ;[0.6848 1 0.5705] Set Team Affiliation for affected Board Tiles
    (for _index (range _teamaffiliationrowcount)
      (for _array_element (`.1DBoard_4_A8DABEF5403C21CC9E4A7485542F37BF` (break `/Game/AlgorithmBoardGame/Blueprints/Structs/F_Board1D` (`|GetArrayItem` (`self.Board2D`) _index)))
        (bind _structout (setmembers `/Game/AlgorithmBoardGame/Blueprints/Structs/F_BoardTile` :`StructRef` _array_element :`TeamAffiliation` 1))
        (`PrimitiveComponent.SetMaterial` (`/Game/AlgorithmBoardGame/Blueprints/BP_Tile.Cube` (`.TileInstance_9_CA27FE9E4DD3D7EA48119F8EA3C33D02` (break `/Game/AlgorithmBoardGame/Blueprints/Structs/F_BoardTile` _structout))) 0 "/Game/AlgorithmBoardGame/Resources/Materials/M_TeamBlue.M_TeamBlue")))
    (for _index_2 (range (- _returnvalue _teamaffiliationrowcount) _returnvalue)
      (for _array_element_2 (`.1DBoard_4_A8DABEF5403C21CC9E4A7485542F37BF` (break `/Game/AlgorithmBoardGame/Blueprints/Structs/F_Board1D` (`|GetArrayItem` (`self.Board2D`) _index_2)))
        (bind _structout_2 (setmembers `/Game/AlgorithmBoardGame/Blueprints/Structs/F_BoardTile` :`StructRef` _array_element_2 :`TeamAffiliation` 2))
        (`PrimitiveComponent.SetMaterial` (`/Game/AlgorithmBoardGame/Blueprints/BP_Tile.Cube` (`.TileInstance_9_CA27FE9E4DD3D7EA48119F8EA3C33D02` (break `/Game/AlgorithmBoardGame/Blueprints/Structs/F_BoardTile` _structout_2))) 0 "/Game/AlgorithmBoardGame/Resources/Materials/M_TeamRed.M_TeamRed")))))

(fn `UserConstructionScript`)
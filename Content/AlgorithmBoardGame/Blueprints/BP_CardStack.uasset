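; BP_CardStack is a Blueprint stack of cards for the algorithm board game.
; It wraps a Cards array as a last-in, first-out container with Push, Pop, Top, Size and IsEmpty functions, treating the last element as the top.
; Pop removes the top card without returning it and prints a warning when empty, while Top returns no card in that case.
; The event graph and construction script hold no logic.
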(fn `IsEmpty`
  (returns (bEmpty :type Boolean))
  (return (`KismetArrayLibrary.Array_IsEmpty` (`self.Cards`))))

(fn `Pop`
  (bind _cards (`self.Cards`))
  (if (`KismetArrayLibrary.Array_IsNotEmpty` _cards)
    (`KismetArrayLibrary.Array_Remove` _cards (`KismetArrayLibrary.Array_LastIndex` _cards))
    (else
      (`KismetSystemLibrary.PrintText` "Stack is empty! Cannot pop"))))

(fn `Push`
  (params (NewCard :type "/Game/AlgorithmBoardGame/Blueprints/BP_Card Object Reference"))
  (`KismetArrayLibrary.Array_Append` (`self.Cards`) (`|MakeArray` NewCard)))

(fn `Size`
  (returns (Size :type Integer))
  (return (`KismetArrayLibrary.Array_Length` (`self.Cards`))))

(fn `Top`
  (returns (TopCard :type "/Game/AlgorithmBoardGame/Blueprints/BP_Card Object Reference"))
  (bind _cards (`self.Cards`))
  (if (`KismetArrayLibrary.Array_IsNotEmpty` _cards)
    (return (`|GetArrayItem` _cards (`KismetArrayLibrary.Array_LastIndex` _cards)))
    (else
      (return null))))

(fn `UserConstructionScript`)
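; BP_DrawPile is the draw pile for the algorithm board game, holding cards in a stack and spawning its paired BP_DiscardPile at BeginPlay.
; DrawCard pops and returns the top card, or passes the discard pile's cards to AddCards when the stack is empty.
; AddCards shuffles the incoming array and appends it to the stack.
; The refill branch neither returns a card nor explicitly clears the discard pile.
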(event `self.ReceiveBeginPlay`
  (bind _returnvalue (`|SpawnActorFromClass` "/Game/AlgorithmBoardGame/Blueprints/BP_DiscardPile.BP_DiscardPile_C" (`self.DiscardTransform`) "Undefined" "MultiplyWithRoot" null null))
  (set `self.DiscardPile` _returnvalue))

(fn `AddCards`
  (params (CardArray :type "Array of /Game/AlgorithmBoardGame/Blueprints/BP_Card Object Reference"))
  (if (`KismetArrayLibrary.Array_IsNotEmpty` CardArray)
    (`KismetArrayLibrary.Array_Shuffle` CardArray)
    (`KismetArrayLibrary.Array_Append` (`/Game/AlgorithmBoardGame/Blueprints/BP_CardStack.Cards` (`self.CardStack`)) CardArray)))

(fn `DrawCard`
  (returns (Card :type "/Game/AlgorithmBoardGame/Blueprints/BP_Card Object Reference"))
  (bind _cardstack (`self.CardStack`))
  (bind _bempty (`/Game/AlgorithmBoardGame/Blueprints/BP_CardStack.IsEmpty` _cardstack))
  (if _bempty
    ;[0.7231 1 0.7157] Add cards from discard pile after shuffling them
    (`self.AddCards` (`/Game/AlgorithmBoardGame/Blueprints/BP_DiscardPile.Cards` (`self.DiscardPile`)))
    (else
      (bind _topcard (`/Game/AlgorithmBoardGame/Blueprints/BP_CardStack.Top` _cardstack))
      (`/Game/AlgorithmBoardGame/Blueprints/BP_CardStack.Pop` _cardstack)
      (return _topcard))))

(fn `UserConstructionScript`)
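; BP_Player represents a player in the algorithm board game, holding a hand of cards.
; PlayCard removes the card at a given index from the hand and finds the draw pile whose class name matches the card's class.
; That pile receives the played card in its discard pile and supplies a replacement, which is appended to the hand.
; The event graph and construction script are empty.
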(fn `PlayCard`
  (params (CardIndex :type Integer))
  (locals (CardPlayed :type "/Game/AlgorithmBoardGame/Blueprints/BP_Card Object Reference"))
  (bind _cards (`/Game/AlgorithmBoardGame/Blueprints/BP_Hand.Cards` (`self.Hand`)))
  (set `local.CardPlayed` (`|GetArrayItem` _cards CardIndex))
  (`KismetArrayLibrary.Array_Remove` _cards CardIndex)
  ;[1 1 1] Draws new card and moves played card into Discard Pile
  (for _array_element (`self.DrawPiles`)
    (if (`KismetStringLibrary.EqualEqual_StrStr` (`.Name_2_48DDDAA541A2D8D3BE85D5A6CEE92F4F` (break `/Game/AlgorithmBoardGame/Blueprints/Structs/F_Class` (`/Game/AlgorithmBoardGame/Blueprints/BP_Card.CardClass` (`local.CardPlayed`)))) (`.Name_2_48DDDAA541A2D8D3BE85D5A6CEE92F4F` (break `/Game/AlgorithmBoardGame/Blueprints/Structs/F_Class` (`/Game/AlgorithmBoardGame/Blueprints/BP_DrawPile.Class` _array_element))))
      (`KismetArrayLibrary.Array_Append` (`/Game/AlgorithmBoardGame/Blueprints/BP_DiscardPile.Cards` (`/Game/AlgorithmBoardGame/Blueprints/BP_DrawPile.DiscardPile` _array_element)) (`|MakeArray` (`local.CardPlayed`)))
      (bind _card (`/Game/AlgorithmBoardGame/Blueprints/BP_DrawPile.DrawCard` _array_element))
      (`KismetArrayLibrary.Array_Append` (`/Game/AlgorithmBoardGame/Blueprints/BP_Hand.Cards` (`self.Hand`)) (`|MakeArray` _card))
      (break)))
  (set `local.CardPlayed` null))

(fn `UserConstructionScript`)